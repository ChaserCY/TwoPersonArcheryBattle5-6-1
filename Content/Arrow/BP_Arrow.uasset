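; Bow arrow projectile with an ice Niagara trail and a launch sound bound to the player bow's fire event.
; Fire adds projectile movement at runtime, scaling speed and gravity by draw strength.
; On authority, its first overlap sticks it to the closest bone, dealing damage with a headshot bonus, or to the hit component, pushing physics objects.
; BP_Aim targets explode, destroy both actors and update the game instance's target count.
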(event `self.ReceiveBeginPlay`
  (bind _asbp_my_game_instance (cast `/Game/Player/BP_MyGameInstance` (`GameplayStatics.GetGameInstance`)))
  (bind _asbp_player_1 (cast `/Game/xiang/BP_Player1` (`self.GetInstigator`)))
  (set `self.As BP My Game Instance` _asbp_my_game_instance)
  (set `self.As BP My Player 1` _asbp_player_1)
  (`PrimitiveComponent.SetCollisionEnabled` (`self.ArrowCollision`) "NoCollision")
  (`NiagaraComponent.SetAsset` (`self.Niagara`) "/Game/ArrowTrail/FX/NS_ArrowTrail_Ice.NS_ArrowTrail_Ice" true)
  (add `/Game/Bow/AC_Bow.OnFireBegin` (`self.GetComponentByClass` (`GameplayStatics.GetPlayerPawn` 0) "/Game/Bow/AC_Bow.AC_Bow_C") (delegate `PlaySound`)))

(event `M_Play`
  (bind _returnvalue (`GameplayStatics.SpawnSoundAttached` "/Game/SoundAssets/LaunchingArrow_Cue.LaunchingArrow_Cue" (`self.ArroeMesh`) "None" (0.0 0.0 0.0) (struct) "KeepRelativeOffset" false 1.0 1.0 0.0 null null))
  (set `self.FlyArrowSound` _returnvalue))

(event `PlaySound`
  (`self.M_Play`))

(event `Fire`
  (params (Direction :type "Vector Structure") (Strength :type "Float (double-precision)"))
  ; 给发射的箭添加移动
  (bind _returnvalue (`AddComponent|NODE_AddProjectileMovementComponent-0`))
  (bind _output_get (set `self.ProjectileMovementRef` _returnvalue))
  (bind _output_get_2 (set `MovementComponent.Velocity` (* Direction (`KismetMathLibrary.Lerp` (`self.MinSpeed`) (`self.MaxSpeed`) Strength)) _output_get))
  (set `self.Velocity` _output_get_2)
  (set `ProjectileMovementComponent.ProjectileGravityScale` (`KismetMathLibrary.Lerp` (`self.MaxGravity`) (`self.MinGravity`) Strength) _output_get)
  (`PrimitiveComponent.SetCollisionEnabled` (`self.ArrowCollision`) "QueryAndPhysics")
  (`self.SetLifeSpan` 10.0))

(event `self.ArrowCollision.OnComponentBeginOverlap`
  (params (OverlappedComponent :type "PrimitiveComponent Object Reference") (OtherActor :type "Actor Object Reference") (OtherComp :type "PrimitiveComponent Object Reference") (OtherBodyIndex :type Integer) (bFromSweep :type Boolean) (SweepResult :type "HitResult Structure (by ref)"))
  (bind (_bblockinghit _binitialoverlap _time _distance _location _impactpoint _normal _impactnormal _physmat _hitactor _hitcomponent) (`GameplayStatics.BreakHitResult` SweepResult))
  (bind _returnvalue (`self.GetComponentByClass` _hitactor "/Script/Engine.SkeletalMeshComponent"))
  (bind (_bonelocation _returnvalue_2) (`SkinnedMeshComponent.FindClosestBone_K2` _returnvalue _location 0.0 false))
  (`/Engine/EditorBlueprintResources/ActorMacros.Switch Has Authority`
    (:`Authority`
      (`|ExecutionSequence`
        (:`then_0`
          (if (!= OtherActor (`self.GetInstigator`))
            (`/Engine/EditorBlueprintResources/StandardMacros.DoOnce` false
              (:`Completed`
                (`ActorComponent.K2_DestroyComponent` (`self.ProjectileMovementRef`))
                (`PrimitiveComponent.SetCollisionEnabled` (`self.ArrowCollision`) "NoCollision")
                (`/Engine/EditorBlueprintResources/StandardMacros.IsValid` _returnvalue
                  (:`Is Valid`
                    (`self.K2_AttachToComponent` _returnvalue _returnvalue_2 "SnapToTarget" "KeepWorld" "KeepWorld")
                    (`|ExecutionSequence`
                      (:`then_0`
                        (if (== _returnvalue_2 "head")
                          (message `/Game/Player/DamagInterface.TakeDamage` _hitactor 90.0)
                          (else
                            (message `/Game/Player/DamagInterface.TakeDamage` _hitactor 30.0)))
                        (`KismetSystemLibrary.Delay` 2.0)
                        (`ActorComponent.K2_DestroyComponent` (`self.Niagara`)))
                      (:`then_1`
                        (bind _asbp_base_monster (cast `/Game/_Li/BP/Source/BP_BaseMonster` _hitactor)
                          (:`then`
                            (`/Game/_Li/BP/Source/BP_BaseMonster.Suffer_damage` _asbp_base_monster 30.0))
                          (:`CastFailed`
                            (`KismetSystemLibrary.PrintString` "Hello"))))))
                  (:`Is Not Valid`
                    (`self.K2_AttachToComponent` _hitcomponent "None" "KeepWorld" "KeepWorld" "KeepWorld")
                    (if (`SceneComponent.IsSimulatingPhysics` _hitcomponent "None")
                      (`PrimitiveComponent.AddImpulse` _hitcomponent (/ (`self.Velocity`) 5.0) "None" true))
                    (`KismetSystemLibrary.Delay` 2.0)
                    (`ActorComponent.K2_DestroyComponent` (`self.Niagara`))))))))
        (:`then_1`
          (bind _asbp_aim (cast `/Game/Background/BP_Aim` _hitactor))
          (`/Engine/EditorBlueprintResources/StandardMacros.IsValid` _asbp_aim
            (:`Is Valid`
              (`GameplayStatics.SpawnEmitterAtLocation` "/Game/Realistic_Starter_VFX_Pack_Vol2/Particles/Explosion/P_Explosion_Big_A.P_Explosion_Big_A" (`SceneComponent.K2_GetComponentLocation` (`self.Scene`)) (struct) (0.7 0.7 0.7))
              (`GameplayStatics.PlaySoundAtLocation` "/Game/SoundAssets/small_explosion2_Cue.small_explosion2_Cue" (`self.K2_GetActorLocation` _hitactor) (struct) 1.0 1.0 0.0 null null null null)
              (`self.K2_DestroyActor` _asbp_aim)
              (`self.K2_DestroyActor` self)
              (`/Game/Player/BP_MyGameInstance.CalculateAimNum` (`self.As BP My Game Instance`)))))))))

(fn `UserConstructionScript`)