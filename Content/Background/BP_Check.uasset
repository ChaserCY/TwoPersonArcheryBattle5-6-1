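; BP_Check is a one-shot trigger box that shows an introduction and sets up aim targets when the player enters it.
; On overlap with BP_MyPlayer_1, it displays the W_Introduce widget briefly, then spawns a BP_Aim at every actor tagged "LC".
; It stores the level's total BP_Aim count in BP_MyGameInstance as AimMaxNum, destroys itself and prints that count.
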(event `self.Box.OnComponentBeginOverlap`
  (params (OverlappedComponent :type "PrimitiveComponent Object Reference") (OtherActor :type "Actor Object Reference") (OtherComp :type "PrimitiveComponent Object Reference") (OtherBodyIndex :type Integer) (bFromSweep :type Boolean) (SweepResult :type "HitResult Structure (by ref)"))
  (bind _asbp_my_player_1 (cast `/Game/Player/BP_MyPlayer_1` OtherActor))
  (`/Engine/EditorBlueprintResources/StandardMacros.IsValid` _asbp_my_player_1
    (:`Is Valid`
      (`/Engine/EditorBlueprintResources/StandardMacros.DoOnce` false
        (:`Completed`
          (bind _returnvalue (`|CreateWidget` "/Game/Widget/W_Introduce.W_Introduce_C"))
          (`UserWidget.AddToViewport` _returnvalue 0)
          (`KismetSystemLibrary.Delay` 5.0)
          (`Widget.RemoveFromParent` _returnvalue)
          (`KismetSystemLibrary.Delay` 1.0)
          (bind _outactors (`GameplayStatics.GetAllActorsWithTag` "LC"))
          (for _array_element _outactors
            (`|SpawnActorFromClass` "/Game/Background/BP_Aim.BP_Aim_C" (`KismetMathLibrary.MakeTransform` (`self.K2_GetActorLocation` _array_element)) "Undefined" "MultiplyWithRoot" null null))
          (bind _outactors_2 (`GameplayStatics.GetAllActorsOfClass` "/Game/Background/BP_Aim.BP_Aim_C"))
          (bind _asbp_my_game_instance (cast `/Game/Player/BP_MyGameInstance` (`GameplayStatics.GetGameInstance`)))
          (bind _output_get (set `/Game/Player/BP_MyGameInstance.AimMaxNum` (`KismetArrayLibrary.Array_Length` _outactors_2) _asbp_my_game_instance))
          (`self.K2_DestroyActor`)
          (`KismetSystemLibrary.PrintString` (`KismetStringLibrary.Conv_IntToString` _output_get)))))))

(fn `UserConstructionScript`)