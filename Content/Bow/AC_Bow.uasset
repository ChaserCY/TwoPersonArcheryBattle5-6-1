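; Bow component for BP_Player1 that handles equipping, aiming, drawing and firing, with server-named events and dispatch calls for each stage.
; It spawns BP_Bow on authority, moving it between hand and back sockets, and spawns a hand-held arrow while aiming.
; A looping timer builds draw time, which switches on a fire trail and sets shot strength.
; A camera trace supplies aim direction; the recoil montage's end re-nocks if still aiming.
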(event `self.ReceiveBeginPlay`
  (bind _asbp_player_1 (cast `/Game/xiang/BP_Player1` (`self.GetOwner`)))
  (set `self.MyPlayerRef` _asbp_player_1)
  (`/Engine/EditorBlueprintResources/ActorComponentMacros.Switch Has Authority`
    (:`Authority`
      (`self.OnServerEquippedBow`))))

(event `OnServerEquippedBow`
  ; 装备弓
  (bind _bow_ref (`self.Bow_Ref`)
    (:`then`
      (`Actor.K2_DetachFromActor` _bow_ref "KeepRelative" "KeepRelative" "KeepRelative")
      (`Actor.K2_AttachToComponent` _bow_ref (`Character.Mesh` (`self.MyPlayerRef`)) "hand_l_Bow" "KeepRelative" "KeepRelative" "KeepRelative" true))
    (:`else`
      (bind _returnvalue (`|SpawnActorFromClass` "/Game/Bow/BP_Bow.BP_Bow_C" (`KismetMathLibrary.MakeTransform` (0.0 0.0 0.0)) "Undefined" "MultiplyWithRoot" null null))
      (bind _output_get (set `self.Bow_Ref` _returnvalue))
      (`Actor.K2_AttachToComponent` _output_get (`Character.Mesh` (`self.MyPlayerRef`)) "hand_l_Bow" "KeepRelative" "KeepRelative" "KeepRelative" true))))

(event `SwitchBow`
  (`self.OnServerEquippedBow`))

(event `OnServerNoBow`
  (bind _bow_ref (`self.Bow_Ref`)
    (:`then`
      (`Actor.K2_DetachFromActor` _bow_ref "KeepRelative" "KeepRelative" "KeepRelative")
      (`Actor.K2_AttachToComponent` _bow_ref (`Character.Mesh` (`self.MyPlayerRef`)) "Back_Bow" "KeepRelative" "KeepRelative" "KeepRelative" true))
    (:`else`)))

(event `NoBow`
  (`self.OnServerNoBow`))

(event `OnServerAimBegin`
  ; 瞄准开始与结束
  (set `self.IsAiming` true)
  (set `/Game/Bow/BP_Bow.BowState` "NewEnumerator1" (`self.Bow_Ref`))
  (`self.OnServerSpawnArrow`)
  (`self.CallOnAimBegin`))

(event `CallOnAimBegin`
  ; 瞄准开始与结束
  (`self.OnAimBegin`))

(event `OnServerAimEnd`
  ; 瞄准开始与结束
  (set `self.IsAiming` false)
  (set `/Game/Bow/BP_Bow.BowState` "NewEnumerator0" (`self.Bow_Ref`))
  (`self.OnServerDestroyAimingArroe`)
  (`self.CallOnAimEnd`)
  (`self.OnServerDrawEnd`))

(event `CallOnAimEnd`
  ; 瞄准开始与结束
  (`self.OnAimEnd`))

(event `OnServerSpawnArrow`
  ; 箭的生成
  (`self.AimingArrowwRef`
    (:`then`)
    (:`else`
      (bind _returnvalue (`|SpawnActorFromClass` "/Game/Arrow/BP_Arrow.BP_Arrow_C" (`KismetMathLibrary.MakeTransform` (0.0 0.0 0.0)) "Undefined" "MultiplyWithRoot" null (`self.MyPlayerRef`)))
      (bind _output_get (set `self.AimingArrowwRef` _returnvalue))
      (`Actor.K2_AttachToComponent` _output_get (`Character.Mesh` (`self.MyPlayerRef`)) "hand_r_Arrow" "SnapToTarget" "SnapToTarget" "SnapToTarget" true))))

(event `OnServerDestroyAimingArroe`
  ; 箭的生成
  (bind _aimingarrowwref (`self.AimingArrowwRef`)
    (:`then`
      (`Actor.K2_DestroyActor` _aimingarrowwref))
    (:`else`)))

(event `CallOnDrawBegin`
  (params (MaxDrawTime :type "Float (double-precision)") (DrawTime :type "Float (double-precision)"))
  ; 蓄力拉弓
  (`self.OnDrawBegin` MaxDrawTime DrawTime))

(event `OnServerDrawBegin`
  ; 蓄力拉弓
  (if (and (`self.IsAiming`) (not (`self.IsDrawing`)) (not (`self.IsFiringArrow`)) (not (`/Game/xiang/BP_Player1.IsRolling` (`self.MyPlayerRef`))))
    (set `self.IsDrawing` true)
    (bind _returnvalue (`KismetSystemLibrary.K2_SetTimerDelegate` (delegate `IncrementDrawTime`) (`self.IcrementTimeRate`) true))
    (set `self.DrawBowTimer` _returnvalue)
    (set `/Game/Bow/BP_Bow.BowState` "NewEnumerator2" (`self.Bow_Ref`))
    (`self.PlayDrawSound`)))

(event `CallOnDrawEnd`
  ; 蓄力拉弓
  (`self.OnDrawEnd`))

(event `IncrementDrawTime`
  ; 蓄力拉弓
  (bind _output_get (set `self.DrawTime` (+ (`self.DrawTime`) (`self.IcrementTimeRate`))))
  (`self.SetNiagara`)
  (`self.CallOnDrawBegin` (`/Game/Bow/BP_Bow.MaxDrawTime` (`self.Bow_Ref`)) _output_get))

(event `SetNiagara`
  ; 蓄力拉弓
  (if (> (`self.DrawTime`) 0.9)
    (`self.AimingArrowwRef`
      (:`then`
        (`NiagaraComponent.SetAsset` (`/Game/Arrow/BP_Arrow.Niagara` (`self.AimingArrowwRef`)) "/Game/ArrowTrail/FX/NS_ArrowTrail_Fire_02.NS_ArrowTrail_Fire_02" true))
      (:`else`))))

(event `PlayDrawSound`
  ; 蓄力拉弓
  (`/Engine/EditorBlueprintResources/StandardMacros.IsValid` (`self.DrawBowSound`)
    (:`Is Not Valid`
      (bind _returnvalue (`GameplayStatics.SpawnSoundAttached` "/Game/SoundAssets/DrawBowSound_Cue.DrawBowSound_Cue" (`/Game/Bow/BP_Bow.BowSkeletalMesh` (`self.Bow_Ref`)) "None" (0.0 0.0 0.0) (struct) "KeepRelativeOffset" false 1.0 1.0 0.0 "/Game/SoundAssets/SA_RunSound.SA_RunSound" null))
      (set `self.DrawBowSound` _returnvalue))))

(event `OnServerDrawEnd`
  ; 蓄力拉弓
  (set `self.IsDrawing` false)
  (set `self.DrawTime` 0.0)
  (`KismetSystemLibrary.K2_ClearAndInvalidateTimerHandle` (`self.DrawBowTimer`))
  (set `/Game/Bow/BP_Bow.BowState` "NewEnumerator0" (`self.Bow_Ref`))
  (`self.CallOnDrawEnd`)
  (`self.StopDrawSound`))

(event `StopDrawSound`
  ; 蓄力拉弓
  (bind _drawbowsound (`self.DrawBowSound`)
    (:`then`
      (`AudioComponent.FadeOut` _drawbowsound 0.1 0.0 "Linear")
      (`self.K2_DestroyComponent` _drawbowsound))
    (:`else`)))

(event `OnServerFireBegin`
  (params (Direction :type "Vector Structure"))
  ; 发射箭矢
  (if (`self.IsDrawing`)
    (set `self.IsFiringArrow` true)
    (bind _aimingarrowwref (`self.AimingArrowwRef`)
      (:`then`
        (`Actor.K2_DetachFromActor` _aimingarrowwref "KeepWorld" "KeepWorld" "KeepWorld")
        (`/Game/Arrow/BP_Arrow.Fire` (`self.AimingArrowwRef`) Direction (`KismetMathLibrary.FClamp` (`KismetMathLibrary.NormalizeToRange` (`self.DrawTime`) 0.0 (`/Game/Bow/BP_Bow.MaxDrawTime` (`self.Bow_Ref`)))))
        (set `self.AimingArrowwRef` null)
        (`self.CallOnFireBegin`)
        (`self.MulticastPlay`)
        (`self.OnServerDrawEnd`))
      (:`else`))))

(event `CallOnFireBegin`
  ; 发射箭矢
  (`self.OnFireBegin`))

(event `MulticastPlay`
  ; 发射箭矢
  (`|PlayMontage` (`Character.Mesh` (`self.MyPlayerRef`)) "/Game/xiang/NewAnimation/ReStanding_Aim_Recoil_Montage.ReStanding_Aim_Recoil_Montage"
    (:`OnCompleted`
      _)
    (:`OnInterrupted`
      _))
  (`self.OnServerFireEnd`))

(event `OnServerFireEnd`
  ; 发射箭矢
  (set `self.IsFiringArrow` false)
  (if (`self.IsAiming`)
    (`self.OnServerAimBegin`)))

(fn `CulculateDirection`
  (returns (Direction :type "Vector Structure"))
  (bind _followcamera (`/Game/xiang/BP_Player1.FollowCamera` (`self.MyPlayerRef`)))
  (bind _returnvalue (`SceneComponent.K2_GetComponentLocation` _followcamera))
  (bind (_outhit _returnvalue_2) (`KismetSystemLibrary.LineTraceSingle` _returnvalue (+ _returnvalue (* (`SceneComponent.GetForwardVector` _followcamera) 10000.0)) "TraceTypeQuery2"))
  (bind _aimingarrowwref (`self.AimingArrowwRef`)
    (:`then`
      (bind (_bblockinghit _binitialoverlap _time _distance _location _impactpoint _normal _impactnormal _physmat _hitactor _hitcomponent _hitbonename _bonename _hititem _elementindex _faceindex _tracestart _traceend) (`GameplayStatics.BreakHitResult` _outhit))
      (return (`KismetMathLibrary.GetDirectionUnitVector` (`Actor.K2_GetActorLocation` _aimingarrowwref) (`KismetMathLibrary.SelectVector` _location _traceend _returnvalue_2))))
    (:`else`)))