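; Game state Blueprint that shows a level-name widget (WBP_Dis) and plays level-specific background music.
; On BeginPlay, after a short delay, the authority picks CurrentBGM from the current level name and crossfades the BGM component via fade out, sound swap and fade in.
; OnRep_CurrentBGM repeats the swap through replication, but its Delayyy call does not hold back the sound change.
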(event `self.ReceiveBeginPlay`
  (bind _bgm (`self.BGM`))
  (bind _bgm_2 (`self.BGM`))
  (bind _bgm_3 (`self.BGM`))
  (`self.UpdateStratUI` (`/Game/Player/BP_MyGameInstance.LevelName` (`/Game/_Li/Map/Map_Help.Get_MyInstance`)))
  (`KismetSystemLibrary.Delay` 0.2)
  (`/Engine/EditorBlueprintResources/ActorMacros.Switch Has Authority`
    (:`Authority`
      (bind _returnvalue (`GameplayStatics.GetCurrentLevelName` true))
      (bind _output_get (set `self.Level Name` _returnvalue))
      (switch `string` _output_get
        (:`Level001`
          (set `self.CurrentBGM` "/Game/_Li/Sound/Level/诡异低沉的氛围_Cue.诡异低沉的氛围_Cue")
          (`AudioComponent.FadeOut` (`self.BGM`) 1.0 0.0 "Linear")
          (`AudioComponent.SetSound` _bgm_2 (`self.CurrentBGM`))
          (`KismetSystemLibrary.Delay` 1.0)
          (`AudioComponent.FadeIn` _bgm_2 1.0 1.0 0.0 "Linear"))
        (:`Level002`
          (set `self.CurrentBGM` "/Game/_Li/Sound/Level/地牢_Cue.地牢_Cue")
          (`AudioComponent.FadeOut` (`self.BGM`) 1.0 0.0 "Linear")
          (`AudioComponent.SetSound` _bgm_3 (`self.CurrentBGM`))
          (`KismetSystemLibrary.Delay` 1.0)
          (`AudioComponent.FadeIn` _bgm_3 1.0 1.0 0.0 "Linear"))
        (:`abbey`
          (set `self.CurrentBGM` "/Game/_Li/Sound/Level/户外环境_Cue.户外环境_Cue")
          (`AudioComponent.FadeOut` (`self.BGM`) 1.0 0.0 "Linear")
          (`AudioComponent.SetSound` _bgm (`self.CurrentBGM`))
          (`KismetSystemLibrary.Delay` 1.0)
          (`AudioComponent.FadeIn` _bgm 1.0 1.0 0.0 "Linear"))))))

(event `UpdateStratUI`
  (params (Level :type Text))
  (bind _returnvalue (`|CreateWidget` "/Game/_Li/Talk/WBP_Dis.WBP_Dis_C" (`GameplayStatics.GetPlayerController` 0) Level))
  (`UserWidget.AddToViewport` _returnvalue 0))

(event `Delayyy`
  (`KismetSystemLibrary.Delay` 1.0))

(fn `OnRep_CurrentBGM`
  (bind _bgm (`self.BGM`))
  (`self.CurrentBGM`
    (:`then`
      (`AudioComponent.FadeOut` (`self.BGM`) 1.0 0.0 "Linear")
      (`self.Delayyy`)
      (`AudioComponent.SetSound` _bgm (`self.CurrentBGM`))
      (`AudioComponent.FadeIn` _bgm 1.0 1.0 0.0 "Linear"))
    (:`else`)))

(fn `UserConstructionScript`)