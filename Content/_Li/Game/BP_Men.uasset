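; BP_Men is a door actor that sinks out of the way when opened, then removes itself.
; Its Open event plays a timeline whose track drives the static mesh's relative Z location downward.
; The actor is destroyed when the timeline finishes.
; Nothing in this graph triggers Open; disconnected leftovers show a tag-based lookup and a delayed self-open.
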(event `self.ReceiveBeginPlay`)

(event `Open`
  (bind (_direction _0_1) (`Timeline|时间轴`)
    (:`Update`
      (`SceneComponent.K2_SetRelativeLocation` (`self.StaticMesh`) (`KismetMathLibrary.MakeVector` 0.0 0.0 (* _0_1 -700.0)) false false))
    (:`Finished`
      (`self.K2_DestroyActor`))))

(fn `UserConstructionScript`)