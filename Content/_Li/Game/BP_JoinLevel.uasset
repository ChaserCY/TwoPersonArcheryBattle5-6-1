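; BP_JoinLevel is a multiplayer level-exit trigger that moves the session to LevelName once all players stand inside its box.
; When IsE is set, the server tracks overlapping BP_Player1 actors and compares their count to the GameState PlayerArray.
; A full zone triggers a fade widget and delayed ServerTravel as listen server; otherwise a notice shows the headcount.
; Optionally, Is3 makes an overlap set the Is3 flag on GetMyInstance.
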(event `self.Box.OnComponentBeginOverlap`
  (params (OverlappedComponent :type "PrimitiveComponent Object Reference") (OtherActor :type "Actor Object Reference") (OtherComp :type "PrimitiveComponent Object Reference") (OtherBodyIndex :type Integer) (bFromSweep :type Boolean) (SweepResult :type "HitResult Structure (by ref)"))
  (bind _returnvalue (`KismetArrayLibrary.Array_Length` (`self.PlayersInZone `)))
  (bind _returnvalue_2 (`KismetArrayLibrary.Array_Length` (`GameStateBase.PlayerArray` (`GameplayStatics.GetGameState`))))
  (if (`self.IsE`)
    (`|ExecutionSequence`
      (:`then_0`
        (if (`self.Is3`)
          (`self.Zu`)))
      (:`then_1`
        (bind _asbp_player_1 (cast `/Game/xiang/BP_Player1` OtherActor))
        (set `self.As BP Player 1` _asbp_player_1)
        (`/Engine/EditorBlueprintResources/ActorMacros.Switch Has Authority`
          (:`Authority`
            (`KismetArrayLibrary.Array_AddUnique` (`self.PlayersInZone `) _asbp_player_1)
            (if (== _returnvalue_2 _returnvalue)
              (`self.Multi_PlayFadeUI`)
              (`KismetSystemLibrary.Delay` 1.5)
              (`KismetSystemLibrary.ExecuteConsoleCommand` (`KismetStringLibrary.Concat_StrStr` "ServerTravel " (`self.LevelName`) "?listen") (`GameplayStatics.GetPlayerController` 0))
              (else
                (`self.Bo` _returnvalue _returnvalue_2)))))))))

(event `Multi_PlayFadeUI`
  (bind _returnvalue (`|CreateWidget` "/Game/_Li/WBP/Level/WBP_Black.WBP_Black_C" (`GameplayStatics.GetPlayerController` 0)))
  (`UserWidget.AddToViewport` _returnvalue 0))

(event `Zu`
  (set `/Game/Player/BP_MyGameInstance.Is3` true (`/Game/_Li/Map/Map_Help.Get_MyInstance`)))

(event `self.Box.OnComponentEndOverlap`
  (params (OverlappedComponent :type "PrimitiveComponent Object Reference") (OtherActor :type "Actor Object Reference") (OtherComp :type "PrimitiveComponent Object Reference") (OtherBodyIndex :type Integer))
  (bind _asbp_player_1 (cast `/Game/xiang/BP_Player1` OtherActor))
  (`/Engine/EditorBlueprintResources/ActorMacros.Switch Has Authority`
    (:`Authority`
      (`KismetArrayLibrary.Array_RemoveItem` (`self.PlayersInZone `) _asbp_player_1))))

(event `Bo`
  (params (Man :type Integer) (SumMan :type Integer))
  (bind _returnvalue (`|CreateWidget` "/Game/_Li/WBP/Level/WBP_Notice.WBP_Notice_C" (`GameplayStatics.GetPlayerController` 0)))
  (`UserWidget.AddToViewport` _returnvalue 0)
  (`/Game/_Li/WBP/Level/WBP_Notice.Set Man` _returnvalue (`KismetTextLibrary.Conv_IntToText` Man) (`KismetTextLibrary.Conv_IntToText` SumMan)))

(fn `UserConstructionScript`)