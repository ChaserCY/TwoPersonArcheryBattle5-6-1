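; BP_Chufa is a trigger box that starts dialogue and can spawn a level-join actor.
; When IsE is set, a locally controlled BP_Player1 overlap shows a Talk1 widget once and stores the level name in the game instance.
; If IsOpen, it also spawns BP_JoinLevel once the game state's PlayerNow equals the player count.
; The similar Date handler's binding and the Players de-duplication check are disconnected.
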(event `Add Player`
  (if (== (`/Game/_Li/Sound/BP_GameState.PlayerNow` (`/Game/_Li/Map/Map_Help.Get_MyGameState`)) (`KismetArrayLibrary.Array_Length` (`GameStateBase.PlayerArray` (`GameplayStatics.GetGameState`))))
    (set `/Game/_Li/Sound/BP_GameState.LevelName` (`self.Level Name_Text`) (`/Game/_Li/Map/Map_Help.Get_MyGameState`))
    (`|SpawnActorFromClass` "/Game/_Li/Game/BP_JoinLevel.BP_JoinLevel_C" (`self.GetTransform` self) "Undefined" "MultiplyWithRoot" null (`self.Level Name`) (`self.Is 3`) null)))

(event `self.Box.OnComponentBeginOverlap`
  (params (OverlappedComponent :type "PrimitiveComponent Object Reference") (OtherActor :type "Actor Object Reference") (OtherComp :type "PrimitiveComponent Object Reference") (OtherBodyIndex :type Integer) (bFromSweep :type Boolean) (SweepResult :type "HitResult Structure (by ref)"))
  (if (`self.IsE`)
    (bind _asbp_player_1 (cast `/Game/xiang/BP_Player1` OtherActor))
    (if (`Pawn.IsLocallyControlled` _asbp_player_1)
      (`|ExecutionSequence`
        (:`then_0`
          (`/Engine/EditorBlueprintResources/StandardMacros.DoOnce` false
            (:`Completed`
              (bind _returnvalue (`|CreateWidget` "/Game/_Li/Talk/Talk1.Talk1_C" (`GameplayStatics.GetPlayerController` 0) (`self.Row Name`)))
              (`UserWidget.AddToViewport` _returnvalue 0)
              (`self.ZU`))))
        (:`then_1`
          (if (`self.IsOpen`)
            (`self.Add Player`)))))))

(event `ZU`
  (set `/Game/Player/BP_MyGameInstance.LevelName` (`self.Level Name_Text`) (`/Game/_Li/Map/Map_Help.Get_MyInstance`)))

(event `Date`
  (bind _asbp_my_game_instance (`/Game/_Li/Map/Map_Help.Get_MyInstance`))
  (`/Engine/EditorBlueprintResources/StandardMacros.IncrementInt` (`self.Num`)
    (:`  `
      (if (== (`/Game/Player/BP_MyGameInstance.PlayerNow` _asbp_my_game_instance) (`/Game/Player/BP_MyGameInstance.PlayerNum` _asbp_my_game_instance))
        (set `/Game/Player/BP_MyGameInstance.LevelName` (`self.Level Name_Text`) (`/Game/_Li/Map/Map_Help.Get_MyInstance`))
        (`|SpawnActorFromClass` "/Game/_Li/Game/BP_JoinLevel.BP_JoinLevel_C" (`self.GetTransform` self) "Undefined" "MultiplyWithRoot" null (`self.Level Name`) (`self.Is 3`) null)))))

(fn `UserConstructionScript`)