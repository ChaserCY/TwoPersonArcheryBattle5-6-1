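; AC_NPCDamage is an actor component that manages replicated health and death for BP_BaseMonster NPCs.
; TakeDamage clamps Health, flags IsDead at zero and returns death state with health ratio.
; OnRep_Health caches the owning monster, updates its health bar widget and plays a hurt sound while alive.
; OnRep_IsDead enables ragdoll physics on the mesh and, on authority, stops the AI controller's brain logic and movement.
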(event `self.ReceiveBeginPlay`)

(fn `OnRep_Health`
  (bind _as_bpc_ai_npc (`self.As BPC AI NPC`))
  (bind _bpw_npchealth (`/Game/_Li/BP/Source/BP_BaseMonster.BPW NPCHealth` (`self.As BPC AI NPC`)))
  (`self.As BPC AI NPC`
    (:`then`
      _)
    (:`else`
      (bind _asbp_base_monster (cast `/Game/_Li/BP/Source/BP_BaseMonster` (`self.GetOwner`)))
      (set `self.As BPC AI NPC` _asbp_base_monster)))
  (`/Engine/EditorBlueprintResources/StandardMacros.IsValid` _bpw_npchealth
    (:`Is Valid`
      (`/Game/_Li/AI/BPW_NPCHealth.UpdateHealthBar` _bpw_npchealth (/ (`self.Health`) (`self.MaxHealth`)))
      (if (> (`self.Health`) 0.0)
        (`GameplayStatics.PlaySoundAtLocation` (`/Game/_Li/BP/Source/BP_BaseMonster.Sound_Hurt` _as_bpc_ai_npc) (`Actor.K2_GetActorLocation` _as_bpc_ai_npc) (struct) 1.0 1.0 0.0 null null null null)))))

(fn `OnRep_IsDead`
  (bind _as_bpc_ai_npc (`self.As BPC AI NPC`))
  (`PrimitiveComponent.SetCollisionEnabled` (`Character.CapsuleComponent` _as_bpc_ai_npc) "QueryAndPhysics")
  (`PrimitiveComponent.SetSimulatePhysics` (`Character.Mesh` _as_bpc_ai_npc) true)
  (`/Engine/EditorBlueprintResources/ActorComponentMacros.Switch Has Authority`
    (:`Authority`
      (bind _asbpac_kzq (cast `/Game/_Li/AI/BPAC_KZQ` (`Pawn.GetController` (`self.As BPC AI NPC`))))
      (`BrainComponent.StopLogic` (`AIController.BrainComponent` _asbpac_kzq) "Death")
      (`Controller.StopMovement` _asbpac_kzq))))

(fn `TakeDamage`
  (params (DamageAmount :type "Float (double-precision)"))
  (returns (IsDead :type Boolean) (PrograessValue :type "Float (double-precision)"))
  (if (not (`self.IsDead`))
    (bind _output_get (set `self.Health` (`KismetMathLibrary.FClamp` (- (`self.Health`) DamageAmount) 0.0 (`self.MaxHealth`))))
    (if (not (> _output_get 0.0))
      (set `self.IsDead` true))
    (return (`self.IsDead`) (/ (`self.Health`) (`self.MaxHealth`)))))