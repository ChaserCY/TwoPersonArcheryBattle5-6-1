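; Base monster for a multiplayer game: attacks players, takes damage and can unlock barriers when killed.
; A data table row supplies stats and montages, ACNPCDamage tracks health for the widget bar, and the server relays struck and attack states to BPAC_KZQ.
; Attacks deal damage after a delay if the target remains close; a proximity box asks players to toggle the bar.
; Tagged deaths increment a GameInstance counter that opens BP_Men or destroys a wall.
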(event `self.ReceiveBeginPlay`
  (`SceneComponent.SetVisibility` (`self.Widget`) false false)
  (`/Engine/EditorBlueprintResources/ActorMacros.Switch Has Authority`
    (:`Authority`
      ; 获取玩家实例列表(只有服务器才能拿到)
      (bind _asbp_my_game_mode (cast `/Game/Player/BP_MyGameMode` (`GameplayStatics.GetGameMode`)))
      (set `self.Players` (`/Game/Player/BP_MyGameMode.Players` _asbp_my_game_mode))
      ; 获取NPC对应的AI控制器实例
      (bind _asbpac_kzq (cast `/Game/_Li/AI/BPAC_KZQ` (`AIBlueprintHelperLibrary.GetAIController` self)))
      (set `self.As BPAC KZQ` _asbpac_kzq))
    (:`Remote`
      _))
  ; 获取NPC血条的控件实例
  (bind _asbpw_npchealth (cast `/Game/_Li/AI/BPW_NPCHealth` (`WidgetComponent.GetWidget` (`self.Widget`))))
  (set `self.BPW NPCHealth` _asbpw_npchealth)
  (set `self.Is_Server` (`self.HasAuthority`))
  (bind _returnvalue (`|GetDataTableRow` (`self.Montage_DataTable`) (`self.Row Name`))
    (:`then`
      (bind (_max_health _gongji _suffer _dying _attack _sound_hurt) (break `/Game/_Li/DataTable/BPS_NPCMontage` _returnvalue))
      (set `/Game/_Li/BP/AC_NPCDamage.MaxHealth` _max_health (`self.AC_NPCDamage`))
      (set `self.Gongji` _gongji)
      (set `self.Sound_Hurt` _sound_hurt))
    (:`RowNotFound`
      (set `/Game/_Li/BP/AC_NPCDamage.MaxHealth` 100.0 (`self.AC_NPCDamage`))
      (set `self.Gongji` 10.0))))

(event `self.ReceiveAnyDamage`
  (params (Damage :type "Float (single-precision)") (DamageType :type "DamageType Object Reference") (InstigatedBy :type "Controller Object Reference") (DamageCauser :type "Actor Object Reference"))
  ; 受到伤害
  (`self.Suffer_damage` Damage))

(event `Suffer_damage`
  (params (Damege :type "Float (double-precision)"))
  ; 受到伤害
  ;; 接口
  (`KismetSystemLibrary.PrintText` (`|FormatText` "受到伤害：{1}" Damege))
  (bind (_isdead _prograessvalue) (`/Game/_Li/BP/AC_NPCDamage.TakeDamage` (`self.AC_NPCDamage`) Damege))
  (bind _bpw_npchealth (`self.BPW NPCHealth`)
    (:`then`
      _)
    (:`else`
      (bind _asbpw_npchealth (cast `/Game/_Li/AI/BPW_NPCHealth` (`WidgetComponent.GetWidget` (`self.Widget`))))
      (set `self.BPW NPCHealth` _asbpw_npchealth)))
  (`/Game/_Li/AI/BPW_NPCHealth.Set_Progress` _bpw_npchealth _prograessvalue)
  (`/Game/_Li/AI/BPW_NPCHealth.Set_Progress` (`self.BPW NPCHealth`) _prograessvalue)
  (`/Engine/EditorBlueprintResources/ActorMacros.Switch Has Authority`
    (:`Authority`
      (if _isdead
        (`self.Death`)
        (`Widget.SetVisibility` (`WidgetComponent.GetWidget` (`self.Widget`)) "Hidden")
        (`self.DestoryActor`)
        (else
          (`self.As BPAC KZQ`
            (:`then`
              _)
            (:`else`
              ; 收到伤害与死亡动画
              (bind _asbpac_kzq (cast `/Game/_Li/AI/BPAC_KZQ` (`AIBlueprintHelperLibrary.GetAIController` self)))
              (set `self.As BPAC KZQ` _asbpac_kzq)))
          (`Controller.StopMovement` (`self.As BPAC KZQ`))
          (`/Game/_Li/AI/BPAC_KZQ.Set_Struck` (`self.As BPAC KZQ`) true)
          (`self.Struck`)
          (`KismetSystemLibrary.Delay` 1.0)
          (`/Game/_Li/AI/BPAC_KZQ.Set_Struck` (`self.As BPAC KZQ`) false))))))

(event `Struck`
  ; 收到伤害与死亡动画
  (bind _returnvalue (`|GetDataTableRow` (`self.Montage_DataTable`) (`self.Row Name`))
    (:`then`
      (`|PlayMontage` (`self.Mesh`) (`.Suffer_3_2E3384664934EEDAE62ACABA2EBF26B7` (break `/Game/_Li/DataTable/BPS_NPCMontage` _returnvalue))))))

(event `DestoryActor`
  ; 销毁时
  (if (`self.HaveTr`)
    (if (`self.ActorHasTag` (`self.Tag`))
      (bind _result (`/Engine/EditorBlueprintResources/StandardMacros.IncrementInt` (`/Game/Player/BP_MyGameInstance.L01_n` (`/Game/_Li/Map/Map_Help.Get_MyInstance`)))
        (:`  `
          (if (>= _result (`self.Ti`))
            (set `/Game/Player/BP_MyGameInstance.L01_n` 0 (`/Game/_Li/Map/Map_Help.Get_MyInstance`))
            (bind _destory_wall (`self.Destory_Wall`)
              (:`then`
                (bind _asbp_men (cast `/Game/_Li/Game/BP_Men` _destory_wall)
                  (:`then`
                    (`/Game/_Li/Game/BP_Men.Open` _asbp_men))
                  (:`CastFailed`
                    (`self.K2_DestroyActor` _destory_wall)
                    (`KismetSystemLibrary.Delay` 5.0 :!label _label)
                    (`self.K2_DestroyActor`))))
              (:`else`
                (goto _label)))
            (else
              (goto _label)))))
      (else
        (goto _label)))))

(event `Death`
  ; 收到伤害与死亡动画
  (bind _returnvalue (`|GetDataTableRow` (`self.Montage_DataTable`) (`self.Row Name`))
    (:`then`
      (`|PlayMontage` (`self.Mesh`) (`.Dying_7_6DCB0BD54C3ACCD4B639EC927900F816` (break `/Game/_Li/DataTable/BPS_NPCMontage` _returnvalue))))))

(event `/Game/_Li/BP/BPI_NPC.Set_AttckState`
  (params (Attck_State :type Boolean))
  ; 修改攻击状态
  (bind _output_get (set `self.Is_Attack` Attck_State))
  (`self.Set_Server_ArrackState` _output_get))

(event `Set_Server_ArrackState`
  (params (Is_Attack :type Boolean))
  ; 修改攻击状态
  (bind _as_bpac_kzq (`self.As BPAC KZQ`)
    (:`then`
      (`/Game/_Li/AI/BPAC_KZQ.Set_Attack` _as_bpac_kzq Is_Attack))
    (:`else`)))

(event `Lanunch Attack`
  (params (`Player Actor` :type "/Game/xiang/BP_Player1 Object Reference") (Damage :type "Float (double-precision)"))
  ; 主动对玩家发起攻击并播放动画
  ;; 接口
  (`self.Attack Animation` `Player Actor`)
  (`KismetSystemLibrary.Delay` 1.0)
  (if (< (`KismetMathLibrary.Vector_Distance` (`self.K2_GetActorLocation` `Player Actor`) (`self.K2_GetActorLocation`)) 230.0)
    (`/Game/xiang/BP_Player1.TakeDamage` `Player Actor` Damage)))

(event `Attack Animation`
  (params (Player_Actor :type "/Game/xiang/BP_Player1 Object Reference"))
  ; 主动对玩家发起攻击并播放动画
  (bind _returnvalue (`|GetDataTableRow` (`self.Montage_DataTable`) (`self.Row Name`))
    (:`then`
      (`|PlayMontage` (`self.Mesh`) (`.Attack_9_FB8045DC4247A08EBD65D78185F93053` (break `/Game/_Li/DataTable/BPS_NPCMontage` _returnvalue)) 1.5
        (:`then`
          (`KismetSystemLibrary.Delay` 0.7))))))

(event `self.Box.OnComponentBeginOverlap`
  (params (OverlappedComponent :type "PrimitiveComponent Object Reference") (OtherActor :type "Actor Object Reference") (OtherComp :type "PrimitiveComponent Object Reference") (OtherBodyIndex :type Integer) (bFromSweep :type Boolean) (SweepResult :type "HitResult Structure (by ref)"))
  ; 近距离显示血条
  (bind _asbp_player_1 (cast `/Game/xiang/BP_Player1` OtherActor))
  (`/Engine/EditorBlueprintResources/ActorMacros.Switch Has Authority`
    (:`Authority`
      (`/Game/xiang/BP_Player1.update vis` _asbp_player_1 self))))

(event `self.Box.OnComponentEndOverlap`
  (params (OverlappedComponent :type "PrimitiveComponent Object Reference") (OtherActor :type "Actor Object Reference") (OtherComp :type "PrimitiveComponent Object Reference") (OtherBodyIndex :type Integer))
  ; 近距离显示血条
  (bind _asbp_player_1 (cast `/Game/xiang/BP_Player1` OtherActor))
  (`/Game/xiang/BP_Player1.update unvis` _asbp_player_1 self))

(fn `Dealth_Destruction`
  (`self.K2_DestroyActor`))

(fn `Get_AttckState`
  (returns (Is_Attck :type Boolean))
  (return (`self.Is_Attack`)))

(fn `Get_Health`
  (returns (Cur_Health :type "Float (double-precision)"))
  (return (`/Game/_Li/BP/AC_NPCDamage.Health` (`self.AC_NPCDamage`))))

(fn `Get_MaxHealth`
  (returns (Max_Health :type "Float (double-precision)"))
  (return (`/Game/_Li/BP/AC_NPCDamage.MaxHealth` (`self.AC_NPCDamage`))))

(fn `Have_dealth`
  (`PrimitiveComponent.SetCollisionEnabled` (`self.CapsuleComponent`) "NoCollision")
  (`/Game/_Li/AI/BPAC_KZQ.Have_Dealth` (`self.As BPAC KZQ`)))

(fn `Set_Health`
  (params (Health :type "Float (double-precision)") (MaxHealth :type "Float (double-precision)"))
  (set `/Game/_Li/BP/AC_NPCDamage.Health` Health (`self.AC_NPCDamage`))
  (set `/Game/_Li/BP/AC_NPCDamage.MaxHealth` MaxHealth (`self.AC_NPCDamage`)))

(fn `Set_Struck`
  (params (BoolValue :type Boolean))
  (`/Game/_Li/AI/BPAC_KZQ.Set_Struck` (`self.As BPAC KZQ`) BoolValue))

(fn `UserConstructionScript`)