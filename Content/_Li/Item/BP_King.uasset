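; BP_King is an item Blueprint whose pickup logic acts as a key for tagged trigger and level-join actors.
; ExecutePickupLogic looks up BP_Chufa and BP_JoinLevel actors tagged "Key" and sets IsE to true on the first of each.
; The lookups have no empty-array check, and BeginPlay, overlap and Tick are disabled stubs.
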(event `self.Execute_Pickup_Logic`
  (params (Player :type "/Game/xiang/BP_Player1 Object Reference"))
  (bind _outactors (`GameplayStatics.GetAllActorsOfClassWithTag` "/Game/_Li/Talk/BP_Chufa.BP_Chufa_C" "Key"))
  (set `/Game/_Li/Talk/BP_Chufa.IsE` true (`|GetArrayItem` _outactors))
  (bind _outactors_2 (`GameplayStatics.GetAllActorsOfClassWithTag` "/Game/_Li/Game/BP_JoinLevel.BP_JoinLevel_C" "Key"))
  (set `/Game/_Li/Game/BP_JoinLevel.IsE` true (`|GetArrayItem` _outactors_2)))

(fn `UserConstructionScript`
  (`parent.UserConstructionScript`))