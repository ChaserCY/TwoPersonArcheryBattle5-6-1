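; BP_Oil is an oil item Blueprint with custom pickup behavior.
; Its ExecutePickupLogic event spawns a BP_BaseItem at an actor's transform and does nothing else.
; BeginPlay, overlap and Tick are disabled stubs, and the construction script only calls the parent.
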(event `self.Execute_Pickup_Logic`
  (params (Player :type "/Game/xiang/BP_Player1 Object Reference"))
  (`|SpawnActorFromClass` "/Game/_Li/Item/BP_BaseItem.BP_BaseItem_C" (`self.GetTransform` (`self.Actor`)) "Undefined" "MultiplyWithRoot" null null))

(fn `UserConstructionScript`
  (`parent.UserConstructionScript`))