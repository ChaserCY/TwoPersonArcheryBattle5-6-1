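; BP_AddBlood is a health pickup item that heals the player who collects it.
; Its ExecutePickupLogic event passes the AddHealth amount to the player's ACDamage component, then prints a debug message and that amount on screen.
; It has no active overlap or tick logic of its own, so pickup triggering comes from outside this graph.
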(event `self.Execute_Pickup_Logic`
  (params (Player :type "/Game/xiang/BP_Player1 Object Reference"))
  (bind _add_health (`self.Add Health`))
  (`/Game/Player/AC_Damage.AddHealth` (`/Game/xiang/BP_Player1.AC_Damage` Player) _add_health)
  (`KismetSystemLibrary.PrintText` "加血了")
  (`KismetSystemLibrary.PrintText` (`KismetTextLibrary.Conv_DoubleToText` _add_health "HalfToEven")))

(fn `UserConstructionScript`
  (`parent.UserConstructionScript`))