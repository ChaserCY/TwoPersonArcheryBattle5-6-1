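; BP_BaseItem is a base actor for items the player can pick up.
; Its Sphere overlap shows the interact prompt and sets itself as TargetItem on a locally controlled BP_Player1 tagged "Player".
; Leaving the sphere hides the prompt and clears TargetItem, without checking whether it still points to this item.
; Execute_Pickup_Logic receives the player but is empty here, apparently a hook for child items.
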(event `self.ReceiveBeginPlay`)

(event `self.Sphere.OnComponentBeginOverlap`
  (params (OverlappedComponent :type "PrimitiveComponent Object Reference") (OtherActor :type "Actor Object Reference") (OtherComp :type "PrimitiveComponent Object Reference") (OtherBodyIndex :type Integer) (bFromSweep :type Boolean) (SweepResult :type "HitResult Structure (by ref)"))
  (if (`self.ActorHasTag` OtherActor "Player")
    (bind _asbp_player_1 (cast `/Game/xiang/BP_Player1` OtherActor))
    (if (`Pawn.IsLocallyControlled` _asbp_player_1)
      (`Widget.SetVisibility` (`/Game/xiang/BP_Player1.HUD_InteractPrompt` _asbp_player_1) "Visible")
      (set `/Game/xiang/BP_Player1.TargetItem` self _asbp_player_1))))

(event `self.Sphere.OnComponentEndOverlap`
  (params (OverlappedComponent :type "PrimitiveComponent Object Reference") (OtherActor :type "Actor Object Reference") (OtherComp :type "PrimitiveComponent Object Reference") (OtherBodyIndex :type Integer))
  (if (`self.ActorHasTag` OtherActor "Player")
    (bind _asbp_player_1 (cast `/Game/xiang/BP_Player1` OtherActor))
    (if (`Pawn.IsLocallyControlled` _asbp_player_1)
      (`Widget.SetVisibility` (`/Game/xiang/BP_Player1.HUD_InteractPrompt` _asbp_player_1) "Hidden")
      (set `/Game/xiang/BP_Player1.TargetItem` null _asbp_player_1))))

(event `Execute_Pickup_Logic`
  (params (Player :type "/Game/xiang/BP_Player1 Object Reference")))

(fn `UserConstructionScript`)