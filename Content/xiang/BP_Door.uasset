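; BP_Door is an interactable door actor that the player toggles open and closed by swinging it 90 degrees in yaw.
; BeginPlay caches the closed and open rotations of DoorPivot.
; Interact calls MC_PlayDoor, which flips IsOpen and plays or reverses the TL_Door timeline to lerp the pivot between them.
; InteractionRange overlaps set or clear CurrentDoor on BP_Player1 as it enters or leaves.
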(event `self.ReceiveBeginPlay`
  ; 门开关形式_xiang
  (set `self.ClosedRotation` (`SceneComponent.RelativeRotation` (`self.DoorPivot`)))
  (set `self.OpenRotation` (`KismetMathLibrary.ComposeRotators` (`self.ClosedRotation`) (`KismetMathLibrary.MakeRotator` 0.0 0.0 90.0))))

(event `MC_PlayDoor`
  ; 门开关形式_xiang
  (if (`self.bIsOpen`)
    (`|ExecutionSequence`
      (:`then_0`
        (set `self.bIsOpen` false))
      (:`then_1`
        (bind (_direction _alpha) (`Timeline|TL_Door` :!via `Reverse` :!label _label)
          (:`Update`
            (`SceneComponent.K2_SetRelativeRotation` (`self.DoorPivot`) (`KismetMathLibrary.RLerp` (`self.ClosedRotation`) (`self.OpenRotation`) _alpha) false false)))))
    (else
      (`|ExecutionSequence`
        (:`then_0`
          (goto _label))
        (:`then_1`
          (set `self.bIsOpen` true))))))

(event `Interact`
  ; 门开关形式_xiang
  (`self.MC_PlayDoor`))

(event `self.InteractionRange.OnComponentBeginOverlap`
  (params (OverlappedComponent :type "PrimitiveComponent Object Reference") (OtherActor :type "Actor Object Reference") (OtherComp :type "PrimitiveComponent Object Reference") (OtherBodyIndex :type Integer) (bFromSweep :type Boolean) (SweepResult :type "HitResult Structure (by ref)"))
  ; 角色开关门判断_xiang
  (bind _asbp_player_1 (cast `/Game/xiang/BP_Player1` OtherActor))
  (set `/Game/xiang/BP_Player1.CurrentDoor` self _asbp_player_1))

(event `self.InteractionRange.OnComponentEndOverlap`
  (params (OverlappedComponent :type "PrimitiveComponent Object Reference") (OtherActor :type "Actor Object Reference") (OtherComp :type "PrimitiveComponent Object Reference") (OtherBodyIndex :type Integer))
  ; 角色开关门判断_xiang
  (bind _asbp_player_1 (cast `/Game/xiang/BP_Player1` OtherActor))
  (set `/Game/xiang/BP_Player1.CurrentDoor` null _asbp_player_1))

(fn `UserConstructionScript`)