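; AC_Mask is an actor component that puts a mask on the BP_Player1 character that owns it.
; On BeginPlay it casts its owner to BP_Player1 and checks that the mesh has a head_mask socket.
; BeginAddMask then spawns a BP_Mask, stores it in MaskRef and attaches it to that socket on the player mesh, keeping relative transforms.
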(event `self.ReceiveBeginPlay`
  (bind _asbp_player_1 (cast `/Game/xiang/BP_Player1` (`self.GetOwner`)))
  (if (`SceneComponent.DoesSocketExist` (`Character.Mesh` _asbp_player_1) "head_mask")
    (`self.BeginAddMask`)))

(event `BeginAddMask`
  (bind _returnvalue (`|SpawnActorFromClass` "/Game/xiang/mask/BP_Mask.BP_Mask_C" (`KismetMathLibrary.MakeTransform` (0.0 0.0 0.0)) "Undefined" "MultiplyWithRoot" null null))
  (bind _output_get (set `self.MaskRef` _returnvalue))
  (`Actor.K2_AttachToComponent` _output_get (`Character.Mesh` (`self.Player1Ref`)) "head_mask" "KeepRelative" "KeepRelative" "KeepRelative" true))