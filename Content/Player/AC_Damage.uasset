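; Player health component that applies damage and healing, with health clamped at the maximum.
; When damage empties health, it increments the game instance's DeadMan count and calls MulticastDeath on the owning BP_Player1.
; Health's RepNotify compares against PriorHealth to play hurt or death HUD feedback for the locally controlled pawn.
; TakeMeleeDamage is an empty stub, and the logic setting IsDead and calling FindWinner is disconnected.
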(event `self.ReceiveBeginPlay`
  (if (`Controller.IsLocalController` (`GameplayStatics.GetPlayerController` 0))
    (bind _asbp_my_player_controller (cast `/Game/Player/BP_MyPlayerController` (`GameplayStatics.GetPlayerController` 0)))
    (set `self.HUDRef` (`/Game/Player/BP_MyPlayerController.HUDRef` _asbp_my_player_controller))
    (set `self.Prior Health` (`self.MaxHealth`))))

(fn `AddHealth`
  (params (AddHealth :type "Float (double-precision)"))
  (bind _returnvalue (+ AddHealth (`self.Health`)))
  (if (`self.IsDead`)
    _
    (elif (>= _returnvalue (`self.MaxHealth`))
      (set `self.Health` (`self.MaxHealth`))
      (else
        (set `self.Health` _returnvalue)))))

(fn `OnRep_Health`
  (bind _hudref (`self.HUDRef`))
  (bind _aspawn (cast `Pawn` (`self.GetOwner`)))
  (if (`Pawn.IsLocallyControlled` _aspawn)
    ; 受伤
    (if (< (`self.Health`) (`self.Prior Health`))
      (set `self.Prior Health` (`self.Health`))
      (if (> (`self.Health`) 0.0)
        (`/Game/Widget/W_MyPlayerHUD.PlayHurted` _hudref)
        (else
          (`/Game/Widget/W_MyPlayerHUD.PlayDeath` _hudref)))
      (else
        ; 回血或者不变
        (set `self.Prior Health` (`self.Health`))))))

(fn `TakeDamage`
  (params (DamageAmount :type "Float (double-precision)") (DamageCauser :type "ActorComponent Object Reference"))
  (if (not (`self.IsDead`))
    (bind _output_get (set `self.Health` (`KismetMathLibrary.FClamp` (- (`self.Health`) DamageAmount) 0.0 (`self.MaxHealth`))))
    (if (> _output_get 0.0)
      (return)
      (else
        (`/Engine/EditorBlueprintResources/StandardMacros.IncrementInt` (`/Game/Player/BP_MyGameInstance.DeadMan` (`/Game/_Li/Map/Map_Help.Get_MyInstance`))
          (:`  `
            (bind _asbp_player_1 (cast `/Game/xiang/BP_Player1` (`self.GetOwner`)))
            (`/Game/xiang/BP_Player1.Multicast_Death` _asbp_player_1)))))))

(fn `TakeMeleeDamage`
  (params (`DamageAmount ` :type "Float (double-precision)") (DamageCauser :type "Actor Object Reference")))