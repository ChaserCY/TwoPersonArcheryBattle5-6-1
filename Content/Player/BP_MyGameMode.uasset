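; Game mode for a two-player match that handles match start, spawn assignment, winner display and restart.
; The second login starts a timer, after which a random player is moved to the Player2 location and given a material change.
; ChoosePlayerStart caches tagged starts in a map, using P1/P2, or P3/P4 when the one-shot Is3 flag is set.
; FindWinner shows the win to players with health remaining, and RestartGame server-travels to Lvl_ThirdPerson after a delay.
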(event `self.K2_PostLogin`
  (params (NewPlayer :type "PlayerController Object Reference"))
  (`KismetArrayLibrary.Array_Add` (`self.Players`) NewPlayer)
  (if (`self.HasGameStarted`)
    _
    (elif (== (`KismetArrayLibrary.Array_Length` (`self.Players`)) 2)
      (`self.StartGame`))))

(event `StartGame`
  (`KismetSystemLibrary.K2_SetTimerDelegate` (delegate `ChoseePlayer2`) 1.0))

(event `ChoseePlayer2`
  (bind _players (`self.Players`))
  (bind _player2location (`self.Player2Location`))
  (bind _returnvalue (`Controller.K2_GetPawn` (`self.Player2RefController`)))
  (set `self.HasGameStarted` true)
  (bind _output_get (set `self.Player2RefController` (`|GetArrayItem` _players (`KismetMathLibrary.RandomIntegerInRange` 0 (- (`KismetArrayLibrary.Array_Length` _players) 1)))))
  (`/Engine/EditorBlueprintResources/StandardMacros.IsValid` _output_get
    (:`Is Valid`
      (`/Engine/EditorBlueprintResources/StandardMacros.IsValid` _returnvalue
        (:`Is Valid`
          (bind _asbp_my_player_1 (cast `/Game/Player/BP_MyPlayer_1` _returnvalue))
          (`self.K2_SetActorLocation` _returnvalue _player2location false false)
          (`/Game/Player/BP_MyPlayer_1.SetPlayerLocation` _asbp_my_player_1 _player2location)
          (`/Game/Player/BP_MyPlayer_1.SetMaterial` _asbp_my_player_1))))
    (:`Is Not Valid`
      (`KismetSystemLibrary.Delay` 1.0)
      (`self.ChoseePlayer2`))))

(event `RestartGame`
  (`KismetSystemLibrary.Delay` 3.0)
  (`KismetSystemLibrary.ExecuteConsoleCommand` "ServerTravel Lvl_ThirdPerson" null))

(event `FindWinner`
  (for _array_element (`self.Players`)
    (bind _asbp_my_player_1 (cast `/Game/Player/BP_MyPlayer_1` (`Controller.K2_GetPawn` _array_element)))
    (if (> (`/Game/Player/AC_Damage.Health` (`/Game/Player/BP_MyPlayer_1.AC_Damage` _asbp_my_player_1)) 0.0)
      (bind _asbp_my_player_controller (cast `/Game/Player/BP_MyPlayerController` _array_element))
      (`/Game/Player/BP_MyPlayerController.ShowWin` _asbp_my_player_controller))))

(fn `ChoosePlayerStart`
  (params (Player :type "Controller Object Reference"))
  (returns (ReturnValue :type "Actor Object Reference"))
  (bind (_value _returnvalue) (`BlueprintMapLibrary.Map_Find` (`self.PlayerSpawnMap`)))
  (bind (_value_2 _returnvalue_2) (`BlueprintMapLibrary.Map_Find` (`self.PlayerSpawnMap`) Player))
  ; 两个出生点打上标签P1,P2
  (if (`self.Is3`)
    (set `self.Is3` false)
    (if _returnvalue
      (return _value)
      (elif (== (`BlueprintMapLibrary.Map_Length` (`self.PlayerSpawnMap`)) 0)
        (bind _outactors (`GameplayStatics.GetAllActorsWithTag` "P3"))
        (bind _output (`|GetArrayItem` _outactors))
        (`BlueprintMapLibrary.Map_Add` (`self.PlayerSpawnMap`) null _output)
        (return _output)
        (else
          (bind _outactors_2 (`GameplayStatics.GetAllActorsWithTag` "P4"))
          (bind _output_2 (`|GetArrayItem` _outactors_2))
          (`BlueprintMapLibrary.Map_Add` (`self.PlayerSpawnMap`) null _output_2)
          (return _output_2))))
    (elif _returnvalue_2
      (return _value_2)
      (elif (== (`BlueprintMapLibrary.Map_Length` (`self.PlayerSpawnMap`)) 0)
        (bind _outactors_3 (`GameplayStatics.GetAllActorsWithTag` "P1"))
        (bind _output_3 (`|GetArrayItem` _outactors_3))
        (`BlueprintMapLibrary.Map_Add` (`self.PlayerSpawnMap`) Player _output_3)
        (return _output_3)
        (else
          (bind _outactors_4 (`GameplayStatics.GetAllActorsWithTag` "P2"))
          (bind _output_4 (`|GetArrayItem` _outactors_4))
          (`BlueprintMapLibrary.Map_Add` (`self.PlayerSpawnMap`) Player _output_4)
          (return _output_4))))))

(fn `UserConstructionScript`)